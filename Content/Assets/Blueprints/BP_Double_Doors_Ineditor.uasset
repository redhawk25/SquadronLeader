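; Sliding double door with a rotating logo lock, opened and closed through the Opendoors and Closedoors events.
; One timeline, played or reversed, rotates the lock, mirrors the door panels' movement and drives motor audio pitch.
; Timeline direction gates click, impact and lock sounds; lock material stops glowing on opening and glows again once closed, when CallDoorCloseEvent fires.
; BeginPlay assigns materials; the construction script sets both doors' translucent sort priority.
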(event Custom|Open%20doors
  (Rendering|Material|SetMaterial (Variables|BP_Double_Doors|GetLock) 0 "/Game/Assets/Materials/M_UE4_Logo_Door.M_UE4_Logo_Door") ; Switch to non-glowing material
  (Audio|SpawnSoundAttached "/Game/Assets/Audio/Door_Unlock_Cue.Door_Unlock_Cue" (Variables|Audio|GetDoor%20Opening%20Audio) "None" "0, 0, 0" "0, 0, 0" "EAttachLocation::KeepRelativeOffset" false 1.0 1.0)
  (Audio|Components|Audio|Play (Variables|Audio|GetDoor%20Opening%20Audio) 0.0)
  (bind (_direction _lock_rotation _doormovement) (Timeline|Open/close Play)
    (:Update
      (Audio|Components|Audio|SetPitchMultiplier (Variables|Audio|GetDoor%20Opening%20Audio) (* _doormovement (Variables|Audio|GetDefault%20Pitch)))
      (Transformation|SetRelativeRotation (Variables|BP_Double_Doors|GetLock) (Math|Rotator|MakeRotator _lock_rotation 0.0 0.0) false false) ; Rotate lock portion
      (Transformation|SetRelativeLocation (Variables|BP_Double_Doors|GetRight%20door) (Math|Vector|MakeVector 0.0 _doormovement 0.0) false false) ; Move doors
      (Transformation|SetRelativeLocation (Variables|BP_Double_Doors|GetLeft%20door) (Math|Vector|MakeVector 0.0 (* _doormovement -1.0) 0.0) false false))
    (:Finished
      (if (Utilities|Enum|Equal(Enum) _direction "Backward") ; If the timeline finished reversing...
        (Rendering|Material|SetMaterial (Variables|BP_Double_Doors|GetLock) 0 "/Game/Assets/Materials/M_UE4_Logo_Doors.M_UE4_Logo_Doors") ; Switch to glowing material
        (Audio|Components|Audio|Stop (Variables|Audio|GetDoor%20Opening%20Audio))
        (Audio|SpawnSoundAttached "/Game/Assets/Audio/Door_Lock_Cue.Door_Lock_Cue" (Variables|Audio|GetDoor%20Opening%20Audio) "None" "0, 0, 0" "0, 0, 0" "EAttachLocation::KeepRelativeOffset" false 1.0 1.0)
        (Default|CallDoorCloseEvent)
        (else
          (Audio|Components|Audio|FadeOut (Variables|Audio|GetDoor%20Opening%20Audio) 0.2 0.0 :!class /Script/Engine.AudioComponent)
          (Audio|SpawnSoundAttached "/Game/Assets/Audio/Door_Impact_Cue.Door_Impact_Cue" (Variables|Audio|GetDoor%20Opening%20Audio) "None" "0, 0, 0" "0, 0, 0" "EAttachLocation::KeepRelativeOffset" false 1.0 1.0))))
    (:Close%20Impact
      (if (Utilities|Enum|Equal(Enum) _direction "Backward") ; If the timeline finished reversing...
        (Audio|SpawnSoundAttached "/Game/Assets/Audio/Door_Impact_Cue.Door_Impact_Cue" (Variables|Audio|GetDoor%20Opening%20Audio) "None" "0, 0, 0" "0, 0, 0" "EAttachLocation::KeepRelativeOffset" false 1.0 1.0)
        (Audio|Components|Audio|FadeOut (Variables|Audio|GetDoor%20Opening%20Audio) 0.2 0.0 :!class /Script/Engine.AudioComponent)))
    (:Start%20Open
      (if (Utilities|Enum|Equal(Enum) _direction "Forward") ; If the timeline finished reversing...
        (Audio|SpawnSoundAttached "/Game/Assets/Audio/Door_StartClick_Cue.Door_StartClick_Cue" (Variables|BP_Double_Doors|GetLock) "None" "0, 0, 0" "0, 0, 0" "EAttachLocation::KeepRelativeOffset" false 1.0 1.0)))))

(event Custom|Close%20doors
  (Audio|Components|Audio|Play (Variables|Audio|GetDoor%20Closing%20Audio) 0.0)
  (Audio|SpawnSoundAttached "/Game/Assets/Audio/Door_StartClick_Cue.Door_StartClick_Cue" (Variables|BP_Double_Doors|GetLock) "None" "0, 0, 0" "0, 0, 0" "EAttachLocation::KeepRelativeOffset" false 1.0 1.0)
  (bind (_direction _lock_rotation _doormovement) (Timeline|Open/close Reverse)
    (:Update
      (Audio|Components|Audio|SetPitchMultiplier (Variables|Audio|GetDoor%20Opening%20Audio) (* _doormovement (Variables|Audio|GetDefault%20Pitch)))
      (Transformation|SetRelativeRotation (Variables|BP_Double_Doors|GetLock) (Math|Rotator|MakeRotator _lock_rotation 0.0 0.0) false false) ; Rotate lock portion
      (Transformation|SetRelativeLocation (Variables|BP_Double_Doors|GetRight%20door) (Math|Vector|MakeVector 0.0 _doormovement 0.0) false false) ; Move doors
      (Transformation|SetRelativeLocation (Variables|BP_Double_Doors|GetLeft%20door) (Math|Vector|MakeVector 0.0 (* _doormovement -1.0) 0.0) false false))
    (:Finished
      (if (Utilities|Enum|Equal(Enum) _direction "Backward") ; If the timeline finished reversing...
        (Rendering|Material|SetMaterial (Variables|BP_Double_Doors|GetLock) 0 "/Game/Assets/Materials/M_UE4_Logo_Doors.M_UE4_Logo_Doors") ; Switch to glowing material
        (Audio|Components|Audio|Stop (Variables|Audio|GetDoor%20Opening%20Audio))
        (Audio|SpawnSoundAttached "/Game/Assets/Audio/Door_Lock_Cue.Door_Lock_Cue" (Variables|Audio|GetDoor%20Opening%20Audio) "None" "0, 0, 0" "0, 0, 0" "EAttachLocation::KeepRelativeOffset" false 1.0 1.0)
        (Default|CallDoorCloseEvent)
        (else
          (Audio|Components|Audio|FadeOut (Variables|Audio|GetDoor%20Opening%20Audio) 0.2 0.0 :!class /Script/Engine.AudioComponent)
          (Audio|SpawnSoundAttached "/Game/Assets/Audio/Door_Impact_Cue.Door_Impact_Cue" (Variables|Audio|GetDoor%20Opening%20Audio) "None" "0, 0, 0" "0, 0, 0" "EAttachLocation::KeepRelativeOffset" false 1.0 1.0))))
    (:Close%20Impact
      (if (Utilities|Enum|Equal(Enum) _direction "Backward") ; If the timeline finished reversing...
        (Audio|SpawnSoundAttached "/Game/Assets/Audio/Door_Impact_Cue.Door_Impact_Cue" (Variables|Audio|GetDoor%20Opening%20Audio) "None" "0, 0, 0" "0, 0, 0" "EAttachLocation::KeepRelativeOffset" false 1.0 1.0)
        (Audio|Components|Audio|FadeOut (Variables|Audio|GetDoor%20Opening%20Audio) 0.2 0.0 :!class /Script/Engine.AudioComponent)))
    (:Start%20Open
      (if (Utilities|Enum|Equal(Enum) _direction "Forward") ; If the timeline finished reversing...
        (Audio|SpawnSoundAttached "/Game/Assets/Audio/Door_StartClick_Cue.Door_StartClick_Cue" (Variables|BP_Double_Doors|GetLock) "None" "0, 0, 0" "0, 0, 0" "EAttachLocation::KeepRelativeOffset" false 1.0 1.0)))))

(event EventBeginPlay
  (bind _left_door (Variables|BP_Double_Doors|GetLeft%20door))
  (bind _lock (Variables|BP_Double_Doors|GetLock))
  (Rendering|Material|SetMaterial _left_door 0 "/Game/Assets/Materials/M_DemoWall_Inst_3.M_DemoWall_Inst_3")
  (Rendering|Material|SetMaterial _left_door 1 "/Game/Assets/Materials/M_GlasDoor_Inst.M_GlasDoor_Inst")
  (Rendering|Material|SetMaterial _lock 1 "/Game/Assets/Materials/M_DemoWall_Inst_3.M_DemoWall_Inst_3")
  (Rendering|Material|SetMaterial _lock 0 "/Game/Assets/Materials/M_UE4_Logo_Doors.M_UE4_Logo_Doors"))

(fn ConstructionScript
  (Rendering|SetTranslucentSortPriority (Variables|BP_Double_Doors|GetLeft%20door) (Variables|Default|GetSort%20Priority)))