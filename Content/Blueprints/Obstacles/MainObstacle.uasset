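; MainObstacle is an obstacle actor with a checkpoint trigger and randomly scattered coins.
; When a Spaceship overlaps the Checkpoint component, it calls PassCheckpoint on the Play game mode; the Spaceship_bot branch does nothing after its cast.
; The construction script runs SpawnCoins, which adds a random number of child actor components at random points inside the CoinsArea1 box.
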(event OnComponentBeginOverlap(Checkpoint)
  (params (OtherActor :type Actor%20Object%20Reference) (OtherComp :type Primitive%20Component%20Object%20Reference) (OtherBodyIndex :type Integer) (bFromSweep :type Boolean) (SweepResult :type Hit%20Result%20Structure%20%28by%20ref%29))
  (Utilities|Casting|CastToSpaceship OtherActor
    (:then
      (bind _asplay (Utilities|Casting|CastToPlay (Game|GetGameMode)))
      (Default|PassCheckpoint _asplay))
    (:CastFailed
      (Utilities|Casting|CastToSpaceship_bot OtherActor))))

(event EventBeginPlay)

(event EventActorBeginOverlap
  (params (OtherActor :type Actor%20Object%20Reference)))

(event EventTick
  (params (DeltaSeconds :type Float%20%28single-precision%29)))

(fn ConstructionScript
  (CallFunction|SpawnCoins))

(fn SpawnCoins
  (bind _coinsarea1 (Variables|Default|GetCoinsArea1))
  (for _index (range 0 (Math|Random|RandomIntegerinRange 1 10))
    (AddComponent|AddChildActorComponent false (Math|Conversions|ToTransform(Vector) (Math|Random|RandomPointinBoundingBox (Variables|/Script/Engine.SceneComponent|GetRelativeLocation _coinsarea1) (Variables|/Script/Engine.BoxComponent|GetBoxExtent _coinsarea1))))))