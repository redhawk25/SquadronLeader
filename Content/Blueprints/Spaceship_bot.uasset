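; Spaceship bot Blueprint that keeps running Points and Meters totals for a ship and reports its speed.
; AddPoints and AddMeters add to their totals and return the new value, while GetPoints reads the score.
; GetSpeed derives speed from the rounded length of the velocity vector.
; Move and the construction script are empty, so the file itself contains no movement or bot behavior.
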(fn ConstructionScript)

(fn AddPoints
  (params (NbPoints :type Integer))
  (bind _output_get (Variables|Default|SetPoints (+ NbPoints (Variables|Default|GetPoints) 0)))
  (return _output_get))

(fn GetPoints
  (return (Variables|Default|GetPoints)))

(fn GetSpeed
  (return (Math|Float|Round (Math|Vector|VectorLength (Transformation|GetVelocity)))))

(fn AddMeters
  (params (NbMeters :type Float%20%28single-precision%29))
  (bind _output_get (Variables|Default|SetMeters (+ NbMeters (Variables|Default|GetMeters))))
  (return _output_get))

(fn Move)