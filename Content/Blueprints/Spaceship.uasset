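; Player spaceship pawn for an auto-runner: it constantly flies along X, with bounded steering, boost and brake inputs.
; Tick drives movement, eases mesh tilt from steering and shifts camera FOV for speed sensation.
; Speed falling to a threshold after a brief startup count triggers explosion and game over through the Play GameMode.
; Teleport spawns and possesses a replacement ship, carrying over max speed and points, then destroys itself.
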(event Custom|DollyZoomEffect
  (bind _returnvalue (Utilities|Time|GetWorldDeltaSeconds))
  (bind _camera (Variables|Default|GetCamera))
  ;[1 1 1] Dolly Zoom Effect (Speed sensation)
  (if (Variables|Default|GetZoomOut)
    (bind _output_get (Variables|Default|SetDesiredZoom 1.1e+02))
    (Variables|/Script/Engine.CameraComponent|SetFieldOfView _camera (Math|Interpolation|FInterpTo (Variables|/Script/Engine.CameraComponent|GetFieldOfView (Variables|Default|GetCamera)) _output_get _returnvalue 2.0))
    (elif (Variables|Default|GetZoomIn)
      (bind _output_get_2 (Variables|Default|SetDesiredZoom 7e+01))
      (Variables|/Script/Engine.CameraComponent|SetFieldOfView _camera (Math|Interpolation|FInterpTo (Variables|/Script/Engine.CameraComponent|GetFieldOfView (Variables|Default|GetCamera)) _output_get_2 _returnvalue 2.0))
      (else
        (bind _output_get_3 (Variables|Default|SetDesiredZoom 9e+01))
        (Variables|/Script/Engine.CameraComponent|SetFieldOfView _camera (Math|Interpolation|FInterpTo (Variables|/Script/Engine.CameraComponent|GetFieldOfView (Variables|Default|GetCamera)) _output_get_3 _returnvalue 2.0))))))

(event Custom|RotationMesh
  (bind _staticmesh (Variables|Default|GetStaticMesh))
  ;[1 1 1] Animation Rotation
  (if (Variables|Default|GetMoveRight)
    (Variables|Default|SetRotationX 1e+01)
    (elif (Variables|Default|GetMoveLeft)
      (Variables|Default|SetRotationX -1e+01)
      (else
        (Variables|Default|SetRotationX 0.0))))
  (if (Variables|Default|GetMoveUp)
    (Variables|Default|SetRotationY 1e+01)
    (elif (Variables|Default|GetMoveDown)
      (Variables|Default|SetRotationY -1e+01)
      (else
        (Variables|Default|SetRotationY 0.0))))
  (bind _output_get (Variables|Default|SetFinalRotation (Math|Rotator|MakeRotator (Variables|Default|GetRotationX) (Variables|Default|GetRotationY) 0.0)))
  (Variables|Default|SetFinalRotation _output_get)
  (Transformation|SetRelativeRotation _staticmesh (Math|Interpolation|RInterpTo (Variables|/Script/Engine.SceneComponent|GetRelativeRotation _staticmesh) (Variables|Default|GetFinalRotation) (Utilities|Time|GetWorldDeltaSeconds) 2.0) false false))

(event Custom|Teleport
  (params (location :type Vector))
  (bind _returnvalue (Transformation|GetActorTransform))
  (bind _floatingpawnmovement (Variables|Default|GetFloatingPawnMovement))
  (bind (_location _rotation _scale) (Math|Transform|BreakTransform _returnvalue))
  ;[1 1 1] Teleport
  (if (not (Variables|Default|Getone))
    (Variables|Default|Setone true)
    (bind _returnvalue_2 (Game|SpawnActorfromClass "Spaceship_C" (Math|Transform|MakeTransform location _rotation _scale) "AdjustIfPossibleButAlwaysSpawn" 0 0))
    (Variables|/Script/Engine.FloatingPawnMovement|SetMaxSpeed (Variables|Spaceship_C|GetFloatingPawnMovement _returnvalue_2) (Class|MovementComponent|GetMaxSpeed _floatingpawnmovement))
    (Pawn|Input|AddMovementInput (Pawn|Components|PawnMovement|GetLastInputVector _floatingpawnmovement) 1.0 false)
    (Variables|Spaceship_C|SetPoints _returnvalue_2 (Variables|Default|GetPoints))
    (Pawn|Possess (Game|GetPlayerController 0) _returnvalue_2)
    (Actor|DestroyActor)
    (bind _asplay (Utilities|Casting|CastToPlay (Game|GetGameMode)))
    (Default|TeleportLeader _asplay)))

(event Custom|Death
  (bind _returnvalue (Transformation|GetActorLocation))
  ;[1 1 1] Death
  (Variables|Default|SetIsDead true)
  (Input|DisableInput 0)
  (Effects|SpawnEmitteratLocation "/Game/StarterContent/Particles/P_Explosion.P_Explosion" _returnvalue)
  (Audio|PlaySoundatLocation 0 _returnvalue)
  (Rendering|SetVisibility (Variables|Default|GetStaticMesh) false false)
  (Utilities|FlowControl|Delay 2.0)
  (bind _asplay (Utilities|Casting|CastToPlay (Game|GetGameMode)))
  (Class|LeaderboardBlueprintLibrary|WriteLeaderboardInteger 0 "None")
  (Default|GameOver _asplay))

(event EventTick
  (params (DeltaSeconds :type Float%20%28single-precision%29))
  ;[1 1 1] AutoRun Forward
  (if (not (Variables|Default|GetIsDead))
    (CallFunction|RotationMesh)
    (Pawn|Input|AddMovementInput "1.000000, 0, 0" 1.0 false)
    (CallFunction|DollyZoomEffect)
    (bind _speed (CallFunction|GetSpeed))
    (bind _totalmeters (CallFunction|AddMeters 0.0001))
    (if (<= _speed (Variables|Default|GetDeathSpeed))
      (if (>= _totalmeters 0.002)
        (CallFunction|Death)))))

(event EventBeginPlay
  ;[1 1 1] Variables
  (Variables|/Script/Engine.FloatingPawnMovement|SetMaxSpeed (Variables|Default|GetFloatingPawnMovement) (Variables|Default|GetMaxSpeedValue)))

(event Input|ActionEvents|InputActionAccelerate
  (params (Key :type Key%20Structure :default "AnyKey"))
  (bind _floatingpawnmovement (Variables|Default|GetFloatingPawnMovement))
  (bind _maxspeedvalue (Variables|Default|GetMaxSpeedValue))
  ;[1 1 1] Accelerate
  (:Pressed
    (Variables|/Script/Engine.FloatingPawnMovement|SetMaxSpeed _floatingpawnmovement (+ _maxspeedvalue (Variables|Default|GetDeltaSpeed)))
    (Variables|Default|SetZoomOut true))
  (:Released
    (Variables|/Script/Engine.FloatingPawnMovement|SetMaxSpeed _floatingpawnmovement _maxspeedvalue)
    (Variables|Default|SetZoomOut false)))

(event Input|ActionEvents|InputActionDecelerate
  (params (Key :type Key%20Structure :default "AnyKey"))
  (bind _floatingpawnmovement (Variables|Default|GetFloatingPawnMovement))
  (bind _maxspeedvalue (Variables|Default|GetMaxSpeedValue))
  ;[1 1 1] Decelerate
  (:Pressed
    (Variables|/Script/Engine.FloatingPawnMovement|SetMaxSpeed _floatingpawnmovement (- _maxspeedvalue (/ (Variables|Default|GetDeltaSpeed) 2.0)))
    (Variables|Default|SetZoomIn true))
  (:Released
    (Variables|/Script/Engine.FloatingPawnMovement|SetMaxSpeed _floatingpawnmovement _maxspeedvalue)
    (Variables|Default|SetZoomIn false)))

(event Input|AxisEvents|InputAxisMoveUp
  (params (AxisValue :type Float%20%28single-precision%29))
  (bind _maxspeedvalue (Variables|Default|GetMaxSpeedValue))
  ;[1 1 1] Movements
  (if (< (.Z (Math|Vector|BreakVector (Transformation|GetActorLocation))) (Variables|Default|GetAltitudeMax))
    (Pawn|Input|AddMovementInput (+ (Math|Vector|MakeVector _maxspeedvalue 0.0 0.0) (Math|Vector|MakeVector 0.0 0.0 _maxspeedvalue)) AxisValue false)
    (Variables|Default|SetMoveUp (> AxisValue 0.0))))

(event Input|AxisEvents|InputAxisMoveDown
  (params (AxisValue :type Float%20%28single-precision%29))
  (bind _maxspeedvalue (Variables|Default|GetMaxSpeedValue))
  ;[1 1 1] Movements
  (Pawn|Input|AddMovementInput (- (Math|Vector|MakeVector _maxspeedvalue 0.0 0.0) (Math|Vector|MakeVector 0.0 0.0 _maxspeedvalue)) AxisValue false)
  (Variables|Default|SetMoveDown (> AxisValue 0.0)))

(event Input|AxisEvents|InputAxisMoveRight
  (params (AxisValue :type Float%20%28single-precision%29))
  (bind _maxspeedvalue (Variables|Default|GetMaxSpeedValue))
  ;[1 1 1] Movements
  (if (< (.Y (Math|Vector|BreakVector (Transformation|GetActorLocation))) (Variables|Default|GetMaxRightPosition))
    (Pawn|Input|AddMovementInput (+ (Math|Vector|MakeVector _maxspeedvalue 0.0 0.0) (Math|Vector|MakeVector 0.0 _maxspeedvalue 0.0)) AxisValue false)
    (Variables|Default|SetMoveRight (> AxisValue 0.0))))

(event Input|AxisEvents|InputAxisMoveLeft
  (params (AxisValue :type Float%20%28single-precision%29))
  (bind _maxspeedvalue (Variables|Default|GetMaxSpeedValue))
  ;[1 1 1] Movements
  (if (< (Variables|Default|GetMaxLeftPosition) (.Y (Math|Vector|BreakVector (Transformation|GetActorLocation))))
    (Pawn|Input|AddMovementInput (- (Math|Vector|MakeVector _maxspeedvalue 0.0 0.0) (Math|Vector|MakeVector 0.0 _maxspeedvalue 0.0)) AxisValue false)
    (Variables|Default|SetMoveLeft (> AxisValue 0.0))))

(fn ConstructionScript)

(fn AddPoints
  (params (NbPoints :type Integer))
  (bind _output_get (Variables|Default|SetPoints (+ NbPoints (Variables|Default|GetPoints) 0)))
  (return _output_get))

(fn GetPoints
  (return (Variables|Default|GetPoints)))

(fn GetSpeed
  (return (Math|Float|Round (Math|Vector|VectorLength (Transformation|GetVelocity)))))

(fn AddMeters
  (params (NbMeters :type Float%20%28single-precision%29))
  (bind _output_get (Variables|Default|SetMeters (+ NbMeters (Variables|Default|GetMeters))))
  (return _output_get))