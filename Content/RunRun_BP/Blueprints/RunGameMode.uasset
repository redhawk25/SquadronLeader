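; Game mode for an endless-runner style game that shows the RunHUD and spawns an opening run of floor tiles at BeginPlay.
; AddFloorTiles spawns a random straight tile at NextSpawnPoint, then chains the next spawn to that tile's attach point.
; AddFloorCurves does the same with curve pieces and resets the straight counter.
; The branch that switches to curves after enough straights is disconnected, so curves never spawn from here.
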(event EventBeginPlay
  (bind _returnvalue (UserInterface|CreateWidget "/Game/RunRun_BP/UMG/RunHUD.RunHUD_C"))
  (UserInterface|Viewport|AddtoViewport _returnvalue 0)
  (for _index (range 1 9)
    (CallFunction|AddFloorTiles)))

(fn ConstructionScript)

(fn AddFloorTiles
  (bind _floortiles (Variables|Default|GetFloorTiles))
  (bind _returnvalue (Game|SpawnActorfromClass (Utilities|Array|Get(acopy) _floortiles (Math|Random|RandomIntegerinRange 0 (Utilities|Array|LastIndex _floortiles))) (Variables|Default|GetNextSpawnPoint) "Undefined" 0 0))
  (bind _asbp_floor_tile (Utilities|Casting|CastToBP_FloorTile _returnvalue))
  (bind _attachpoint (Default|GetAttachPoint _asbp_floor_tile))
  (Variables|Default|SetNextSpawnPoint _attachpoint)
  (Variables|Default|SetCurrentStraights (+ (Variables|Default|GetCurrentStraights) 1)))

(fn AddFloorCurves
  (bind _floorcurves (Variables|Default|GetFloorCurves))
  (bind _returnvalue (Game|SpawnActorfromClass (Utilities|Array|Get(acopy) _floorcurves (Math|Random|RandomIntegerinRange 0 (Utilities|Array|LastIndex _floorcurves))) (Variables|Default|GetNextSpawnPoint) "Undefined" 0 0))
  (bind _asbp_floor_tile (Utilities|Casting|CastToBP_FloorTile _returnvalue))
  (bind _attachpoint (Default|GetAttachPoint _asbp_floor_tile))
  (Variables|Default|SetNextSpawnPoint _attachpoint)
  (Variables|Default|SetCurrentStraights 0))