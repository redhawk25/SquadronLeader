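; Canyon floor tile for an endless runner that exposes an attach point transform and randomly populates itself on construction.
; Construction spawns either one blocker at a left, right or middle spawn point, or several coins scattered within a box.
; A Spaceship overlapping the end trigger makes RunGameMode add tiles, then this tile destroys itself after a delay.
; Wall hits kill the ship only when its forward vector nearly matches the hit normal.
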(event OnComponentBeginOverlap(EndTrigger)
  (params (OtherActor :type Actor%20Object%20Reference) (OtherComp :type Primitive%20Component%20Object%20Reference) (OtherBodyIndex :type Integer) (bFromSweep :type Boolean) (SweepResult :type Hit%20Result%20Structure%20%28by%20ref%29))
  ;[1 1 1] Create the road
  (Utilities|Casting|CastToSpaceship OtherActor)
  (bind _asrun_game_mode (Utilities|Casting|CastToRunGameMode (Game|GetGameMode)))
  (Default|AddFloorTiles _asrun_game_mode)
  (Utilities|FlowControl|Delay 2.0)
  (Actor|DestroyActor))

(event OnComponentHit(Wall)
  (params (OtherActor :type Actor%20Object%20Reference) (OtherComp :type Primitive%20Component%20Object%20Reference) (NormalImpulse :type Vector :default "0, 0, 0") (Hit :type Hit%20Result%20Structure%20%28by%20ref%29))
  ;[1 1 1] Hit walls
  (bind _asspaceship (Utilities|Casting|CastToSpaceship OtherActor))
  (if (Math|Float|NearlyEqual(Float) (Math|Vector|DotProduct (Transformation|GetActorForwardVector _asspaceship) (.normal Hit)) 1.0 0.01)
    (Default|Death _asspaceship)))

(event OnComponentHit(Wall2)
  (params (OtherActor :type Actor%20Object%20Reference) (OtherComp :type Primitive%20Component%20Object%20Reference) (NormalImpulse :type Vector :default "0, 0, 0") (Hit :type Hit%20Result%20Structure%20%28by%20ref%29))
  ;[1 1 1] Hit walls
  (bind _asspaceship (Utilities|Casting|CastToSpaceship OtherActor))
  (if (Math|Float|NearlyEqual(Float) (Math|Vector|DotProduct (Transformation|GetActorForwardVector _asspaceship) (.normal Hit)) 1.0 0.01)
    (Default|Death _asspaceship)))

(fn ConstructionScript
  (CallFunction|GetSpawnPoints)
  (switch int (Math|Random|RandomIntegerinRange 0 1)
    (:Default
      (CallFunction|SpawnBlocker :!label _label))
    (:0
      (goto _label))
    (:1
      (CallFunction|SpawnCoins))))

(fn GetAttachPoint
  (return (Transformation|GetWorldTransform (Variables|Components|GetAttachPoint))))

(fn GetSpawnPoints
  (Variables|Default|SetSpawnPoints (Utilities|Array|MakeArray (Transformation|GetRelativeTransform (Variables|Default|GetSpawnPoint)) (Transformation|GetRelativeTransform (Variables|Default|GetSpawnPointL)) (Transformation|GetRelativeTransform (Variables|Default|GetSpawnPointR)))))

(fn SpawnBlocker
  (bind _spawnpoints (Variables|Default|GetSpawnPoints))
  (AddComponent|AddChildActorComponent false (Utilities|Array|Get(acopy) _spawnpoints (Math|Random|RandomIntegerinRange 0 (Utilities|Array|LastIndex _spawnpoints)))))

(fn SpawnCoins
  (bind _coinsarea (Variables|Default|GetCoinsArea))
  (for _index (range 0 (Math|Random|RandomIntegerinRange 1 10))
    (AddComponent|AddChildActorComponent false (Math|Conversions|ToTransform(Vector) (Math|Random|RandomPointinBoundingBox (Variables|/Script/Engine.SceneComponent|GetRelativeLocation _coinsarea) (Variables|/Script/Engine.BoxComponent|GetBoxExtent _coinsarea))))))